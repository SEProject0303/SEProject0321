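; BP_Character is the player character, handling movement, look input and interaction with world objects.
; Move steers along actor axes, or ThirdPersonCamera axes when a head-mounted display is enabled.
; An InteractionCapsule notifies Interactable actors through interface messages as they enter and leave its radius.
; Pressing E starts conversation and releasing E requests item pickup, each messaging only the first overlapping Interactable.
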(event `InputAxis|MoveForward` :consume false :overrideparent false
  (params (AxisValue :type "Float (single-precision)"))
  ;[1 1 1] 移动控制
  (`self.Move` AxisValue (stale `InputAxis|MoveRight` AxisValue) :!label _label))

(event `InputAxis|MoveRight` :consume false :overrideparent false
  (params (AxisValue :type "Float (single-precision)"))
  ;[1 1 1] 移动控制
  (goto _label))

(event `InputAxis|Turn` :overrideparent false
  (params (AxisValue :type "Float (single-precision)"))
  ;[1 1 1] 视角控制
  (`self.AddControllerYawInput` AxisValue))

(event `InputAxis|LookUp` :overrideparent false
  (params (AxisValue :type "Float (single-precision)"))
  ;[1 1 1] 视角控制
  (`self.AddControllerPitchInput` AxisValue)
  (`KismetSystemLibrary.PrintString` "0"))

(event `self.InteractionCapsule.OnComponentBeginOverlap`
  (params (OverlappedComponent :type "PrimitiveComponent Object Reference") (OtherActor :type "Actor Object Reference") (OtherComp :type "PrimitiveComponent Object Reference") (OtherBodyIndex :type Integer) (bFromSweep :type Boolean) (SweepResult :type "HitResult Structure (by ref)"))
  ;[1 1 1] On Begin/End Overlap
  (if (`KismetSystemLibrary.DoesImplementInterface` OtherActor "/Game/SEProject/SEBluePrint/SECharacter/Interactable.Interactable_C")
    (message `/Game/SEProject/SEBluePrint/SECharacter/Interactable.OnEnterPlayerRadius` OtherActor self)))

(event `self.InteractionCapsule.OnComponentEndOverlap`
  (params (OverlappedComponent :type "PrimitiveComponent Object Reference") (OtherActor :type "Actor Object Reference") (OtherComp :type "PrimitiveComponent Object Reference") (OtherBodyIndex :type Integer))
  ;[1 1 1] On Begin/End Overlap
  (if (`KismetSystemLibrary.DoesImplementInterface` OtherActor "/Game/SEProject/SEBluePrint/SECharacter/Interactable.Interactable_C")
    (message `/Game/SEProject/SEBluePrint/SECharacter/Interactable.OnLeavePlayerRadius` OtherActor self)))

(event `Key|E`
  (params (Key :type "Key Structure"))
  ;[1 1 1] E to interact
  (:`Pressed`
    (`self.CheckConversation`))
  (:`Released`
    (`self.GetItem`)))

(fn `CheckConversation`
  (for _array_element (`PrimitiveComponent.GetOverlappingActors` (`self.InteractionCapsule`) null)
    (if (`KismetSystemLibrary.DoesImplementInterface` _array_element "/Game/SEProject/SEBluePrint/SECharacter/Interactable.Interactable_C")
      (message `/Game/SEProject/SEBluePrint/SECharacter/Interactable.TakeConverse` _array_element self)
      (break))))

(fn `GetItem`
  (for _array_element (`PrimitiveComponent.GetOverlappingActors` (`self.InteractionCapsule`) null)
    (if (`KismetSystemLibrary.DoesImplementInterface` _array_element "/Game/SEProject/SEBluePrint/SECharacter/Interactable.Interactable_C")
      (message `/Game/SEProject/SEBluePrint/SECharacter/Interactable.GetItem` _array_element)
      (break))))

(fn `Move`
  (params (MoveForeard :type "Float (double-precision)") (MoveRight :type "Float (double-precision)"))
  (`self.AddMovementInput` (select `bool` (`HeadMountedDisplayFunctionLibrary.IsHeadMountedDisplayEnabled`) :`false` (`self.GetActorForwardVector`) :`true` (`SceneComponent.GetForwardVector` (`self.ThirdPersonCamera`))) MoveForeard)
  (`self.AddMovementInput` (select `bool` (`HeadMountedDisplayFunctionLibrary.IsHeadMountedDisplayEnabled`) :`false` (`self.GetActorRightVector`) :`true` (`SceneComponent.GetRightVector` (`self.ThirdPersonCamera`))) MoveRight))

(fn `UserConstructionScript`)