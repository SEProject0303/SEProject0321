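; BP_AICharacter is a wandering NPC the player can talk to, showing an interaction widget within the player's radius.
; TakeConverse opens a talk widget fed PeopleID and TimeID, disables movement on both characters, shows the cursor and locks camera spin.
; EndTalk re-arms talking and restores walking only on the passed-in character, plus cursor and camera state.
; Tick uses a Delay to issue periodic AIMoveTo calls to random nearby reachable points.
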(event `/Game/SEProject/SEBluePrint/Character/Interactable.OnEnterPlayerRadius`
  (params (Character :type "/Game/SEProject/SEBluePrint/Character/BP_Character Object Reference"))
  ;[1 1 1] On Enter/Leave Player Radius
  (`SceneComponent.SetVisibility` (`self.InteractionWidget`) true false))

(event `/Game/SEProject/SEBluePrint/Character/Interactable.OnLeavePlayerRadius`
  (params (Character :type "/Game/SEProject/SEBluePrint/Character/BP_Character Object Reference"))
  ;[1 1 1] On Enter/Leave Player Radius
  (`SceneComponent.SetVisibility` (`self.InteractionWidget`) false false))

(event `/Game/SEProject/SEBluePrint/Character/Interactable.TakeConverse`
  (params (Character :type "/Game/SEProject/SEBluePrint/Character/BP_Character Object Reference"))
  ;[1 1 1] On Interact With
  (if (`self.CanTalk`)
    (`/Game/SEProject/SEBluePrint/UMG/Talkinterface.ConversationConverse` Character (`self.PeopleID`) (`self.TimeID`))
    (set `self.CanTalk` false)))

(event `/Game/SEProject/SEBluePrint/Character/Interactable.EndTalk`
  (params (Character :type "/Game/SEProject/SEBluePrint/Character/BP_Character Object Reference"))
  ;[1 1 1] 结束对话
  (set `self.CanTalk` true)
  (set `PlayerController.bShowMouseCursor` false (`GameplayStatics.GetPlayerController` 0))
  (`CharacterMovementComponent.SetMovementMode` (`Character.CharacterMovement` Character) "MOVE_Walking" 0)
  (bind _asbp_character (cast `/Game/SEProject/SEBluePrint/Character/BP_Character` (`GameplayStatics.GetPlayerCharacter` 0)))
  (set `/Game/SEProject/SEBluePrint/Character/BP_Character.CanSpinCamera` true _asbp_character))

(event `/Game/SEProject/SEBluePrint/UMG/Talkinterface.ConversationConverse`
  (params (character :type "Character Object Reference") (people :type Integer) (time :type Integer))
  ;[1 1 1] Talk widget
  (`KismetSystemLibrary.PrintString` "Level")
  (bind _returnvalue (`|CreateWidget` "/Game/SEProject/SEBluePrint/UMG/BP_UserWidgetTalk.BP_UserWidgetTalk_C"))
  (set `/Game/SEProject/SEBluePrint/UMG/BP_UserWidgetTalk.PeopleID` people _returnvalue)
  (set `/Game/SEProject/SEBluePrint/UMG/BP_UserWidgetTalk.TimeID` time _returnvalue)
  (`UserWidget.AddToViewport` _returnvalue 0)
  (`Widget.SetVisibility` _returnvalue "Visible")
  (`CharacterMovementComponent.DisableMovement` (`Character.CharacterMovement` character))
  (`CharacterMovementComponent.DisableMovement` (`self.CharacterMovement`))
  (set `PlayerController.bShowMouseCursor` true (`GameplayStatics.GetPlayerController` 0))
  (bind _asbp_character (cast `/Game/SEProject/SEBluePrint/Character/BP_Character` (`GameplayStatics.GetPlayerCharacter` 0)))
  (set `/Game/SEProject/SEBluePrint/Character/BP_Character.CanSpinCamera` false _asbp_character))

(event `self.ReceiveTick`
  (params (DeltaSeconds :type "Float (single-precision)"))
  ;[1 1 1] AI Movement
  (`KismetSystemLibrary.Delay` 3.0)
  (`|AIMoveTo` self (`NavigationSystemV1.K2_GetRandomReachablePointInRadius` (`self.K2_GetActorLocation`) 500.0 null null) null))

(fn `GetID`)

(fn `TickConversation`)

(fn `UserConstructionScript`)