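; BP_AICharacter is an NPC character that shows an interaction widget and can be talked to.
; On BeginPlay it writes its Name into the InteractionWidget component's widget.
; Player-radius enter and leave events toggle that component's visibility.
; TakeConverse calls TickConversation, a placeholder that only prints a debug string, and GetID has an empty body.
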(event `self.ReceiveBeginPlay`
  ;[1 1 1] 设置NPC名字
  (bind _asinteraction_widget (cast `/Game/SEProject/SECharacter/InteractionWidget` (`WidgetComponent.GetUserWidgetObject` (`self.InteractionWidget`))))
  (`TextBlock.SetText` (`/Game/SEProject/SECharacter/InteractionWidget.Name` _asinteraction_widget) (`self.Name`)))

(event `/Game/SEProject/SECharacter/Interactable.OnEnterPlayerRadius`
  (params (Character :type "/Game/SEProject/SECharacter/BP_Character Object Reference"))
  ;[1 1 1] On Enter/Leave Player Radius
  (`SceneComponent.SetVisibility` (`self.InteractionWidget`) true false))

(event `/Game/SEProject/SECharacter/Interactable.OnLeavePlayerRadius`
  (params (Character :type "/Game/SEProject/SECharacter/BP_Character Object Reference"))
  ;[1 1 1] On Enter/Leave Player Radius
  (`SceneComponent.SetVisibility` (`self.InteractionWidget`) false false))

(event `/Game/SEProject/SECharacter/Interactable.TakeConverse`
  (params (Character :type "/Game/SEProject/SECharacter/BP_Character Object Reference"))
  ;[1 1 1] On Interact With
  (`self.TickConversation`))

(fn `GetID`)

(fn `TickConversation`
  (`KismetSystemLibrary.PrintString` "Tick Conveersation"))

(fn `UserConstructionScript`)